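; Cooking station minigame actor where the player clicks to cut a chicken and puts its organs and ingredients into a pot.
; The first chicken click swaps in a cut mesh and shows a random organ; the second enables physics and copies component tags onto the food.
; Pot overlaps destroy ingredients, while one organ mesh respawns from a shrinking random pool.
; Each deposit advances a boolean requirements array toward CompleteMinigame, currently a print stub.
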(event OnClicked(ChickenMesh)
  (params (TouchedComponent :type Primitive%20Component%20Object%20Reference) (ButtonPressed :type Key%20Structure :default "None"))
  (if (Variables|Default|GetCut)
    (Collision|SetCollisionResponsetoChannel (Variables|Components|GetChicken%20Mesh) "ECC_Visibility" "ECR_Ignore")
    (for _array_element (Variables|Default|GetFoodModels)
      (Physics|SetSimulatePhysics _array_element true)
      (Physics|SetEnableGravity _array_element true)
      (Variables|/Script/Engine.ActorComponent|SetComponentTags _array_element (Variables|Default|GetComponent%20Tags)))
    (else
      (Variables|Default|SetCut true)
      (Components|StaticMesh|SetStaticMesh (Variables|Components|GetChicken%20Mesh) "/Game/Models/chicken/chicken_cut1.chicken_cut1")
      (CallFunction|RandomOrgan))))

(event OnComponentBeginOverlap(OrganMesh)
  (params (OverlappedComponent :type Primitive%20Component%20Object%20Reference) (OtherActor :type Actor%20Object%20Reference) (OtherComp :type Primitive%20Component%20Object%20Reference) (OtherBodyIndex :type Integer) (bFromSweep :type Boolean) (SweepResult :type Hit%20Result%20Structure%20%28by%20ref%29))
  ;[0.15 0.15 0.15 0.5] Organs in Pot
  (if (== OtherComp (Variables|Default|GetBox))
    (Rendering|SetVisibility (Variables|Default|GetOrganMesh) false false)
    (Transformation|SetWorldLocationAndRotation (Variables|Default|GetOrganMesh) (Transformation|GetWorldLocation (Variables|Default|GetOrgan%20Spawn)) "0, 0, 0" false false)
    (if (Utilities|Array|IsEmpty (Variables|Default|GetOrgan%20Models))
      (Components|DestroyComponent (Variables|Default|GetOrganMesh))
      (else
        (CallFunction|RandomOrgan)))
    (CallFunction|IncreaseComplete)))

(event OnComponentBeginOverlap(Box)
  (params (OverlappedComponent :type Primitive%20Component%20Object%20Reference) (OtherActor :type Actor%20Object%20Reference) (OtherComp :type Primitive%20Component%20Object%20Reference) (OtherBodyIndex :type Integer) (bFromSweep :type Boolean) (SweepResult :type Hit%20Result%20Structure%20%28by%20ref%29))
  ;[0.15 0.15 0.15 0.5] Food Put in Pot
  (if (Math|Boolean|ORBoolean (== OtherComp (Variables|Default|GetCarrotMesh)) (== OtherComp (Variables|Default|GetOnionMesh)) (== OtherComp (Variables|Default|GetSaltMesh)) (== OtherComp (Variables|Default|GetPepperMesh)))
    (Components|DestroyComponent OtherComp)
    (CallFunction|IncreaseComplete)))

(event OnEndCursorOver(Border)
  (params (TouchedComponent :type Primitive%20Component%20Object%20Reference)))

(event Custom|StartGame
  (bind _returnvalue (Game|GetPlayerController 0))
  (Variables|/Script/Engine.PlayerController|SetbEnableMouseOverEvents _returnvalue true)
  (Variables|/Script/Engine.PlayerController|SetbEnableClickEvents _returnvalue true)
  (Variables|/Script/Engine.PlayerController|SetbShowMouseCursor _returnvalue true))

(event EventBeginPlay
  (bind _returnvalue (Actor|GetActorOfClass "/Game/Blueprints/BP_Main.BP_Main_C"))
  (Variables|Default|SetGrabbed%20Component (Variables|/Game/Blueprints/BP_Main.BP_Main_C|GetGrabbed%20Component _returnvalue)))

(event Collision|EventActorBeginOverlap
  (params (OtherActor :type Actor%20Object%20Reference)))

(event EventTick
  (params (DeltaSeconds :type Float%20%28single-precision%29)))

(fn ConstructionScript
  (bind _foodmodels (Variables|Default|GetFoodModels))
  (Utilities|Array|SetArrayElem _foodmodels 0 (Variables|Default|GetSaltMesh) true)
  (Utilities|Array|SetArrayElem _foodmodels 1 (Variables|Default|GetPepperMesh) true)
  (Utilities|Array|SetArrayElem _foodmodels 2 (Variables|Default|GetCarrotMesh) true)
  (Utilities|Array|SetArrayElem _foodmodels 3 (Variables|Default|GetOnionMesh) true)
  (Utilities|Array|SetArrayElem _foodmodels 4 (Variables|Default|GetOrganMesh) true))

(fn RandomOrgan
  (bind _organmesh (Variables|Default|GetOrganMesh))
  (bind _output_get (LocalVariables|SetLocalindex (.OutIndex (Utilities|Array|Random (Variables|Default|GetOrgan%20Models)))))
  (Components|StaticMesh|SetStaticMesh _organmesh (Utilities|Array|Get(acopy) (Variables|Default|GetOrgan%20Models) _output_get))
  (Rendering|SetVisibility _organmesh true false)
  (Utilities|Array|RemoveItem (Variables|Default|GetOrgan%20Models) (Utilities|Array|Get(acopy) (Variables|Default|GetOrgan%20Models) _output_get)))

(fn IncreaseComplete
  (bind (_array_element _array_index) (Utilities|Array|ForEachLoopwithBreak (Variables|Default|GetRequirements) :!label _label)
    (:LoopBody
      (bind _output_get (LocalVariables|SetLocalIndex _array_index))
      (if (== _array_element false)
        (Utilities|Array|SetArrayElem (Variables|Default|GetRequirements) _output_get true)
        (goto _label Break)
        (else
          _)))
    (:Completed
      _))
  (if (== (+ (LocalVariables|GetLocalIndex) 1) (Utilities|Array|Length (Variables|Default|GetRequirements)))
    (CallFunction|CompleteMinigame)))

(fn CompleteMinigame
  (Development|PrintString "Hello"))