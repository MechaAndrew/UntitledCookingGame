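; Player actor that runs the intro dialogue, then hands off to the cooking station and lets the player drag food with the mouse.
; Space advances lines in a WB_Dialogue widget, swapping character and background art at set indices.
; When lines run out, it attaches its camera to BP_CookingStation's camera and starts the game.
; While the station's Cut flag is set, cursor traces grab "Pickup"-tagged components via PhysicsHandle at their hit distance.
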(event EventBeginPlay
  (bind _returnvalue (Actor|GetActorOfClass "/Game/Blueprints/BP_CookingStation.BP_CookingStation_C"))
  (Variables|Default|SetCookingBP _returnvalue)
  (Variables|/Script/Engine.PlayerController|SetbShowMouseCursor (Game|GetPlayerController 0) false)
  (Default|Talk self)
  (Variables|Default|GetUI%20Dialogue
    (:then)
    (:else
      (bind _returnvalue_2 (UserInterface|CreateWidget "/Game/Blueprints/WB_Dialogue.WB_Dialogue_C" (Game|GetPlayerController 0)))
      (bind _output_get (Variables|Default|SetUI%20Dialogue _returnvalue_2))
      (UserInterface|Viewport|AddtoViewport _output_get 0)
      (Input|SetInputModeUIOnly (Game|GetPlayerController 0) _output_get "DoNotLock" false))))

(event EventTick
  (params (DeltaSeconds :type Float%20%28single-precision%29))
  (bind _returnvalue (Game|GetPlayerController 0))
  (bind (_worldlocation _worlddirection) (Game|Player|ConvertMouseLocationToWorldSpace _returnvalue))
  ;[0.15 0.15 0.15 0.5] Update grab
  (if (Variables|/Game/Blueprints/BP_CookingStation.BP_CookingStation_C|GetCut (Variables|Default|GetCookingBP))
    (bind _grabbed_component (Variables|Default|GetGrabbed%20Component)
      (:then
        (if (Physics|IsSimulatingPhysics _grabbed_component "None")
          (Physics|Components|PhysicsHandle|SetTargetLocation (Variables|Default|GetPhysicsHandle) (+ _worldlocation (* _worlddirection (Variables|Default|GetDistance%20of%20Grabbed%20Organ))))))
      (:else))))

(event EventTalk
  (if (< (Variables|Default|GetDialogue_Index) (Utilities|Array|Length (Variables|Default|GetDialogue)))
    (Variables|Default|GetUI%20Dialogue
      (:then
        _)
      (:else
        (bind _returnvalue (UserInterface|CreateWidget "/Game/Blueprints/WB_Dialogue.WB_Dialogue_C" (Game|GetPlayerController 0)))
        (bind _output_get (Variables|Default|SetUI%20Dialogue _returnvalue))
        (UserInterface|Viewport|AddtoViewport _output_get 0)))
    (Variables|/Script/UMG.TextBlock|SetText (Variables|/Game/Blueprints/WB_Dialogue.WB_Dialogue_C|GetDialogueMain (Variables|Default|GetUI%20Dialogue)) (Utilities|Text|ToText(String) (Utilities|Array|Get(acopy) (Variables|Default|GetDialogue) (Variables|Default|GetDialogue_Index))))
    (bind _result (Math|Integer|IncrementInt (Variables|Default|GetDialogue_Index))
      (:%20%20
        (switch int _result
          (:1
            (CallFunction|UpdateConversationPngs "/Game/UI/Characters/Rebecca/Daughter_Concept_NoBackground.Daughter_Concept_NoBackground" "/Game/UI/Characters/Rebecca/mama_Concept.mama_Concept" "/Game/UI/Elise_Environment/Bed_Room-Final.Bed_Room-Final"))
          (:2
            (CallFunction|UpdateConversationPngs "/Game/UI/Characters/Rebecca/Daughter_Concept.Daughter_Concept" "/Game/UI/Characters/Rebecca/mama_Concept_Transparent.mama_Concept_Transparent" "/Game/UI/Elise_Environment/Bed_Room_Other_Version/BedRoom2.BedRoom2"))
          (:4
            (CallFunction|UpdateConversationPngs "/Game/UI/Characters/Rebecca/Dada_Concept_NonBG.Dada_Concept_NonBG" "/Game/UI/Characters/Rebecca/Daughter_Concept.Daughter_Concept" "/Game/UI/Elise_Environment/Bed_Room_Other_Version/BedRoom4.BedRoom4")))))
    (else
      (Transformation|AttachComponentToComponent (Variables|Default|GetCamera) (Variables|/Game/Blueprints/BP_CookingStation.BP_CookingStation_C|GetCamera (Variables|Default|GetCookingBP)) "None" "KeepRelative" "KeepRelative" "KeepRelative" true)
      (Widget|RemovefromParent (Variables|Default|GetUI%20Dialogue))
      (Default|StartGame (Variables|Default|GetCookingBP)))))

(event Input|MouseEvents|LeftMouseButton
  (params (Key :type Key%20Structure :default "None"))
  (bind _returnvalue (Game|GetPlayerController 0))
  (bind _cookingbp (Variables|Default|GetCookingBP))
  (bind (_worldlocation _worlddirection) (Game|Player|ConvertMouseLocationToWorldSpace _returnvalue))
  (bind _cut (Variables|/Game/Blueprints/BP_CookingStation.BP_CookingStation_C|GetCut _cookingbp))
  ;[0.15 0.15 0.15 0.5] Grab Food
  (:Pressed
    (if _cut
      (bind (_outhit _returnvalue_2) (Collision|LineTraceByChannel _worldlocation (+ _worldlocation (* _worlddirection 1e+04)) "TraceTypeQuery1" false 0 "ForDuration"))
      (if (and _returnvalue_2 (== (.HitActor (Collision|BreakHitResult _outhit)) (Variables|Default|GetCookingBP)))
        (if (== (Utilities|Array|Get(acopy) (Variables|/Script/Engine.ActorComponent|GetComponentTags (.HitComponent (Collision|BreakHitResult _outhit)))) "Pickup")
          (Variables|Default|SetDistance%20of%20Grabbed%20Organ (.Distance (Collision|BreakHitResult _outhit)))
          (bind _output_get (Variables|Default|SetGrabbed%20Component (.HitComponent (Collision|BreakHitResult _outhit))))
          (if (Physics|IsSimulatingPhysics _output_get "None")
            (Class|PhysicsHandleComponent|GrabComponentatLocation (Variables|Default|GetPhysicsHandle) (Variables|Default|GetGrabbed%20Component) "None" (.Location (Collision|BreakHitResult _outhit))))))))
  (:Released
    (if _cut
      (Variables|Default|SetGrabbed%20Component 0)
      (Physics|Components|PhysicsHandle|ReleaseComponent (Variables|Default|GetPhysicsHandle)))))

(event Input|KeyboardEvents|SpaceBar
  (params (Key :type Key%20Structure :default "None"))
  (:Pressed
    (Default|Talk self)
    (Variables|Default|GetUI%20Dialogue
      (:then)
      (:else
        (bind _returnvalue (UserInterface|CreateWidget "/Game/Blueprints/WB_Dialogue.WB_Dialogue_C" (Game|GetPlayerController 0)))
        (bind _output_get (Variables|Default|SetUI%20Dialogue _returnvalue))
        (UserInterface|Viewport|AddtoViewport _output_get 0)
        (Input|SetInputModeUIOnly (Game|GetPlayerController 0) _output_get "DoNotLock" false)))))

(fn ConstructionScript)

(fn UpdateConversationPngs
  (params (Ch1%20IMG :type Texture%202D%20Object%20Reference) (Ch2%20IMG :type Texture%202D%20Object%20Reference) (BG :type Texture%202D%20Object%20Reference))
  (bind _ui_dialogue (Variables|Default|GetUI%20Dialogue))
  (Appearance|SetBrushfromTexture (Variables|/Game/Blueprints/WB_Dialogue.WB_Dialogue_C|GetCharacter1_IMG _ui_dialogue) Ch1%20IMG false)
  (Appearance|SetBrushfromTexture (Variables|/Game/Blueprints/WB_Dialogue.WB_Dialogue_C|GetCharacter2_IMG _ui_dialogue) Ch2%20IMG false)
  (Appearance|SetBrushfromTexture (Variables|/Game/Blueprints/WB_Dialogue.WB_Dialogue_C|GetBackground _ui_dialogue) BG false))